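; Halliste is a player-controlled pawn Blueprint that handles mouse look and keyboard movement.
; Mouse axes feed controller yaw and pitch, scaled by the Sensibilité variable.
; Keyboard axes drive forward/back and right/left movement along directions built from the control rotation's yaw only, so looking up or down leaves movement horizontal.
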(event `InputAxis|Mouse - X`
  (params (AxisValue :type "Float (single-precision)"))
  ;[1 1 1] souris
  (`self.AddControllerYawInput` (* AxisValue (`self.sensibilité`))))

(event `InputAxis|Mouse - Y `
  (params (AxisValue :type "Float (single-precision)"))
  ;[1 1 1] souris
  (`self.AddControllerPitchInput` (* AxisValue (`self.sensibilité`))))

(event `InputAxis|KeyBoard - FB`
  (params (AxisValue :type "Float (single-precision)"))
  ;[1 1 1] clavier
  (`self.AddMovementInput` (`KismetMathLibrary.GetForwardVector` (`KismetMathLibrary.MakeRotator` 0.0 0.0 (.yaw (`self.GetControlRotation`)))) AxisValue))

(event `InputAxis|KeyBoard - RL`
  (params (AxisValue :type "Float (single-precision)"))
  ;[1 1 1] clavier
  (`self.AddMovementInput` (`KismetMathLibrary.GetRightVector` (`KismetMathLibrary.MakeRotator` 0.0 0.0 (.yaw (`self.GetControlRotation`)))) AxisValue))

(fn `UserConstructionScript`)